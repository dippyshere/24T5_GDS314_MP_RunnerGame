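; BP_vine_5 is a spline-driven vine Blueprint from the jungle pack that builds its geometry in the construction script.
; It bends a configurable mesh along each segment of Spline1 with spline mesh components, matching point locations and tangents.
; Two further passes place SM_vine_6 and SM_vine_7 static meshes along the spline, each at its own spacing and oriented to the curve.
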(fn ConstructionScript
  (bind _spacing (Variables|Default|GetSpacing))
  (bind _spacing_0 (Variables|Default|Getspacing_0))
  (bind _spline1 (Variables|Default|GetSpline1))
  (Utilities|FlowControl|Sequence
    (:then_0
      (for _index (range 0 (- (Spline|GetNumberOfSplinePoints _spline1) 2))
        (bind _returnvalue (AddComponent|AddSplineMeshComponent true))
        (Components|StaticMesh|SetStaticMesh _returnvalue (Variables|Default|GetNewVar_0))
        (Rendering|Material|SetMaterial _spline1 0 0)
        (SplineMesh|SetForwardAxis _returnvalue (Variables|Default|Getaxis) true)
        (Transformation|AttachComponentToComponent _returnvalue _spline1 "" "KeepRelative" "KeepRelative" "KeepRelative" true)
        (SplineMesh|SetStartandEnd _returnvalue (Spline|GetLocationatSplinePoint _spline1 _index "Local") (Spline|GetTangentatSplinePoint _spline1 _index "Local") (Spline|GetLocationatSplinePoint _spline1 (+ _index 1 0) "Local") (Spline|GetTangentatSplinePoint _spline1 (+ _index 1 0) "Local") true :!class /Script/Engine.SplineMeshComponent)))
    (:then_1
      (for _index_2 (range 0 (.ReturnValue (Math|Float|Division(WholeandRemainder) (Spline|GetSplineLength _spline1) _spacing)))
        (bind _returnvalue_2 (AddComponent|AddStaticMeshComponent false (Math|Transform|MakeTransform (Spline|GetLocationatDistanceAlongSpline _spline1 (* _index_2 _spacing) "Local") (Spline|GetRotationatDistanceAlongSpline _spline1 (* _index_2 _spacing) "Local"))))
        (Components|StaticMesh|SetStaticMesh _returnvalue_2 "/Game/Jungle_pack/foliage/SM_vine_6.SM_vine_6")))
    (:then_2
      (for _index_3 (range 0 (.ReturnValue (Math|Float|Division(WholeandRemainder) (Spline|GetSplineLength _spline1) _spacing_0)))
        (bind _returnvalue_3 (AddComponent|AddStaticMeshComponent false (Math|Transform|MakeTransform (Spline|GetLocationatDistanceAlongSpline _spline1 (* _index_3 _spacing_0) "Local") (Spline|GetRotationatDistanceAlongSpline _spline1 (* _index_3 _spacing_0) "Local"))))
        (Components|StaticMesh|SetStaticMesh _returnvalue_3 "/Game/Jungle_pack/foliage/SM_vine_7.SM_vine_7")))))